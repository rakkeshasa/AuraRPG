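; Gameplay ability for an enemy ranged attack that turns the avatar toward its combat target and fires a projectile at it.
; On activation it passes the target's location to motion warping and plays a random tagged attack montage.
; When the montage's gameplay event tag arrives, it re-reads the target's location and spawns a projectile from the montage's socket tag, with optional pitch override.
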(event Ability|EventActivateAbility
  (bind _returnvalue (Ability|GetAvatarActorfromActorInfo))
  ;[1 1 1] 고블린이 공격시 캐릭터를 바로보도록
  (bind _returnvalue_2 (Class|EnemyInterface|GetCombatTarget(Message) _returnvalue)) ; Behavior Tree에서 전투 대상을 가져옴
  (Class|CombatInterface|UpdateFacingTarget(Message) _returnvalue (Transformation|GetActorLocation _returnvalue_2)) ; Motion Warping
  (bind _returnvalue_3 (Class|CombatInterface|GetAttackMontages(Message) (Ability|GetAvatarActorfromActorInfo)))
  (bind _output_get (Variables|Default|SetTaggedMontage (Class|AuraDamageGameplayAbility|GetRandomTaggedMontagefromArray _returnvalue_3)))
  (|PlayMontageandWaitProxy "None" (.Montage (Utilities|Struct|BreakTaggedMontage _output_get)) 1.0 "None" false 1.0 0.0
    (:then
      (Ability|Tasks|WaitGameplayEvent (.MontageTag (Utilities|Struct|BreakTaggedMontage _output_get)) 0 true
        (:EventReceived
          (bind _returnvalue_4 (Class|EnemyInterface|GetCombatTarget(Message) (Ability|GetAvatarActorfromActorInfo)))
          (Class|AuraProjectileSpell|SpawnProjectile (Transformation|GetActorLocation _returnvalue_4) (.SocketTag (Utilities|Struct|BreakTaggedMontage _output_get)) (Variables|Default|GetShouldOverride%20Pitch) (Variables|Default|GetPitchOverride)))))))